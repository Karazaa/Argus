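; Debug visual actor for a flying Argus ECS entity, reacting to selection, faction, team, death and passenger events.
; Each event forwards to a small function that updates a component after a validity check.
; Selection toggles the circle, faction name fills the text render, and team color or death grey goes to the cube's custom primitive data.
; Becoming a passenger hides the whole actor; vacating reveals it and deselects it.
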(event EventOnPopulateFaction
  (params (factionRecord :type Faction%20Record%20Object%20Reference))
  ;[1 0 0] Debug functionality
  (NativeEvents|OnPopulateFactionBP factionRecord))

(event EventOnPopulateTeam
  (params (teamColor :type Color%20Structure))
  ;[1 0 0] Debug functionality
  (NativeEvents|OnPopulateTeamBP teamColor))

(event EventOnSelected
  ;[1 0 0] Debug functionality
  (NativeEvents|OnSelectedBP))

(event EventOnDeselected
  ;[1 0 0] Debug functionality
  (NativeEvents|OnDeselectedBP))

(event EventOnArgusEntityDeath
  ;[1 0 0] Debug functionality
  (NativeEvents|OnArgusEntityDeathBP))

(event EventOnArgusEntityPassengerStateChanged
  (params (isPassenger :type Boolean))
  ;[1 0 0] Debug functionality
  (if isPassenger
    (NativeEvents|OnBecomePassengerBP)
    (else
      (NativeEvents|OnVacateCarrierBP)
      (NativeEvents|OnDeselectedBP))))

(fn ConstructionScript)

(fn OnSelectedBP
  ;[1 0 0] Debug functionality
  (bind _selection_circle (Variables|Default|GetSelection%20Circle)
    (:then
      (Development|SetHiddeninGame _selection_circle false true))
    (:else)))

(fn OnDeselectedBP
  ;[1 0 0] Debug functionality
  (bind _selection_circle (Variables|Default|GetSelection%20Circle)
    (:then
      (Development|SetHiddeninGame _selection_circle true true))
    (:else)))

(fn OnPopulateFactionBP
  (params (Faction%20Record :type Faction%20Record%20Object%20Reference))
  ;[1 0 0] Debug functionality
  (bind _textrender (Variables|Default|GetTextRender)
    (:then
      (bind _faction_record (LocalVariables|GetFaction%20Record)
        (:then
          (Rendering|Components|TextRender|SetText _textrender (Utilities|Text|ToText(String) (Variables|/Script/Argus.FactionRecord|Getm_factionName _faction_record))))
        (:else
          (Rendering|Components|TextRender|SetText _textrender (Utilities|Text|ToText(String) "")))))
    (:else)))

(fn OnPopulateTeamBP
  (params (Team%20Color :type Color%20Structure))
  (bind _returnvalue (Math|Conversions|ToLinearColor(Color) Team%20Color))
  (bind (_r _g _b _a) (Utilities|Struct|BreakLinearColor _returnvalue))
  ;[1 0 0] Debug functionality
  (bind _cube (Variables|Default|GetCube)
    (:then
      (Rendering|Material|SetCustomPrimitiveDataVector4 _cube 0 (Math|Vector4|MakeVector4 _r _g _b _a)))
    (:else)))

(fn OnArgusEntityDeathBP
  ;[1 0 0] Debug functionality
  (bind _cube (Variables|Default|GetCube)
    (:then
      (Rendering|Material|SetCustomPrimitiveDataVector4 _cube 0 (Math|Vector4|MakeVector4 0.15 0.15 0.15 1.0)))
    (:else)))

(fn OnBecomePassengerBP
  ;[1 0 0] Debug functionality
  (bind _rootcomponent (Variables|Transformation|GetRootComponent)
    (:then
      (Development|SetHiddeninGame _rootcomponent true true))
    (:else)))

(fn OnVacateCarrierBP
  ;[1 0 0] Debug functionality
  (bind _rootcomponent (Variables|Transformation|GetRootComponent)
    (:then
      (Development|SetHiddeninGame _rootcomponent false true))
    (:else)))
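; Carrier entity actor Blueprint for the Argus ECS, providing debug visuals for selection, faction, team and death.
; Entity events forward to small handlers that toggle components, showing a ground decal when landed or a circle component when flying.
; Team color is written to the Cone's custom primitive data and turns dark gray on death, while a text render shows the faction name.
; Take-off and landing swap the selection indicators without checking whether the carrier is selected.
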(event EventOnPopulateFaction
  (params (factionRecord :type Faction%20Record%20Object%20Reference))
  ;[1 0 0] Debug functionality
  (NativeEvents|OnPopulateFactionBP factionRecord))

(event EventOnTakeOff
  ;[1 0 0] Debug functionality
  (NativeEvents|OnTakeOffBP))

(event EventOnPopulateTeam
  (params (teamColor :type Color%20Structure))
  ;[1 0 0] Debug functionality
  (NativeEvents|OnPopulateTeamBP teamColor))

(event EventOnSelected
  ;[1 0 0] Debug functionality
  (NativeEvents|OnSelectedBP))

(event EventOnDeselected
  ;[1 0 0] Debug functionality
  (NativeEvents|OnDeselectedBP))

(event EventOnArgusEntityDeath
  ;[1 0 0] Debug functionality
  (NativeEvents|OnArgusEntityDeathBP))

(event EventOnLand
  ;[1 0 0] Debug functionality
  (NativeEvents|OnLandBP))

(fn ConstructionScript)

(fn OnSelectedBP
  ;[1 0 0] Debug functionality
  (if (Class|ArgusActor|IsFlying)
    (bind _selection_circle_decal (Variables|Default|GetSelection%20Circle%20Decal)
      (:then
        (Development|SetHiddeninGame _selection_circle_decal true true))
      (:else
        _))
    (bind _selection_circle (Variables|Default|GetSelection%20Circle)
      (:then
        (Development|SetHiddeninGame _selection_circle false true))
      (:else))
    (else
      (bind _selection_circle_decal_2 (Variables|Default|GetSelection%20Circle%20Decal)
        (:then
          (Development|SetHiddeninGame _selection_circle_decal_2 false true))
        (:else
          _))
      (bind _selection_circle_2 (Variables|Default|GetSelection%20Circle)
        (:then
          (Development|SetHiddeninGame _selection_circle_2 true true))
        (:else)))))

(fn OnDeselectedBP
  ;[1 0 0] Debug functionality
  (bind _selection_circle_decal (Variables|Default|GetSelection%20Circle%20Decal)
    (:then
      (Development|SetHiddeninGame _selection_circle_decal true true))
    (:else
      _))
  (bind _selection_circle (Variables|Default|GetSelection%20Circle)
    (:then
      (Development|SetHiddeninGame _selection_circle true true))
    (:else)))

(fn OnPopulateFactionBP
  (params (FactionRecord :type Faction%20Record%20Object%20Reference))
  ;[1 0 0] Debug functionality
  (bind _textrender (Variables|Default|GetTextRender)
    (:then
      (bind _factionrecord (LocalVariables|GetFactionRecord)
        (:then
          (Rendering|Components|TextRender|SetText _textrender (Utilities|Text|ToText(String) (Variables|/Script/Argus.FactionRecord|Getm_factionName _factionrecord))))
        (:else
          (Rendering|Components|TextRender|SetText _textrender (Utilities|Text|ToText(String) "")))))
    (:else)))

(fn OnPopulateTeamBP
  (params (TeamColor :type Color%20Structure))
  (bind _returnvalue (Math|Conversions|ToLinearColor(Color) TeamColor))
  (bind (_r _g _b _a) (Utilities|Struct|BreakLinearColor _returnvalue))
  ;[1 0 0] Debug functionality
  (bind _cone (Variables|Default|GetCone)
    (:then
      (Rendering|Material|SetCustomPrimitiveDataVector4 _cone 0 (Math|Vector4|MakeVector4 _r _g _b _a)))
    (:else)))

(fn OnArgusEntityDeathBP
  ;[1 0 0] Debug functionality
  (bind _cone (Variables|Default|GetCone)
    (:then
      (Rendering|Material|SetCustomPrimitiveDataVector4 _cone 0 (Math|Vector4|MakeVector4 0.15 0.15 0.15 1.0)))
    (:else)))

(fn OnTakeOffBP
  ;[1 0 0] Debug functionality
  (bind _selection_circle_decal (Variables|Default|GetSelection%20Circle%20Decal)
    (:then
      (Development|SetHiddeninGame _selection_circle_decal true true))
    (:else
      _))
  (bind _selection_circle (Variables|Default|GetSelection%20Circle)
    (:then
      (Development|SetHiddeninGame _selection_circle false true))
    (:else)))

(fn OnLandBP
  ;[1 0 0] Debug functionality
  (bind _selection_circle_decal (Variables|Default|GetSelection%20Circle%20Decal)
    (:then
      (Development|SetHiddeninGame _selection_circle_decal false true))
    (:else
      _))
  (bind _selection_circle (Variables|Default|GetSelection%20Circle)
    (:then
      (Development|SetHiddeninGame _selection_circle true true))
    (:else)))